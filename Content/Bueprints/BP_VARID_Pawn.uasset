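; Pawn that drives the VARID plugin, starting its rendering with the first JSON profile found in the plugin's Profiles folder and ending it on End Play.
; Each tick it feeds VARID per-eye gaze from the headset's stereo eye tracker, scaled by a sensitivity value, or falls back to normalised, centred mouse position.
; Number keys toggle individual effects, while comma and period enable or disable all of them.
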(event EventBeginPlay
  ;[1 1 1] Begin Play : Setup VARID
  (Utilities|FlowControl|Sequence
    (:then_0
      ;;[1 1 1] Core
      (Class|VARIDBlueprintFunctionLibrary|SetDisplayFOV (Math|Vector2D|MakeVector2D 106.0 1.1e+02))
      (Class|VARIDBlueprintFunctionLibrary|SetProfileExtension "json")
      (Class|VARIDBlueprintFunctionLibrary|SetProfileRootPath (Utilities|String|Append (Class|BlueprintPathsLibrary|ProjectPluginsDir) "VARID/Content/Profiles/")))
    (:then_1
      ;;[1 1 1] Load Initial Profile
      (bind _outfiles (Class|VARIDBlueprintFunctionLibrary|ListProfiles))
      (if (> (Utilities|Array|Length _outfiles) 0)
        (bind (_profile _returnvalue) (Class|VARIDBlueprintFunctionLibrary|LoadProfile (Utilities|Array|Get(acopy) _outfiles)))
        (if _returnvalue
          (Class|VARIDBlueprintFunctionLibrary|SetActiveProfile _profile))))
    (:then_2
      ;;[1 1 1] Begin Rendering
      (Class|VARIDBlueprintFunctionLibrary|BeginRendering)
      (Actor|Tick|SetActorTickEnabled true))))

(event EventTick
  (params (DeltaSeconds :type Float%20%28single-precision%29))
  ;[1 1 1] Tick : Eye Tracking
  (if (Math|Boolean|ANDBoolean (Class|HeadMountedDisplayFunctionLibrary|IsHeadMountedDisplayEnabled) (Class|EyeTrackerFunctionLibrary|IsStereoGazeDataAvailable) (Class|EyeTrackerFunctionLibrary|IsEyeTrackerConnected))
    (bind _eye_data (CallFunction|VARIDGetEyePositionsfromEyeTracker))
    (Variables|Default|SetEye%20Tracking%20State _eye_data)
    (else
      (bind _eye_data_2 (CallFunction|VARIDGetEyePositionsfromMouse))
      (Variables|Default|SetEye%20Tracking%20State _eye_data_2)))
  (Class|VARIDBlueprintFunctionLibrary|SetEyeTracking (Variables|Default|GetEye%20Tracking%20State)))

(event EventEndPlay
  (params (EndPlayReason :type EEndPlayReason%20Enum :default "Destroyed"))
  ;[1 1 1] End Play : Clean up VARID
  (Utilities|FlowControl|Sequence
    (:then_0
      (Class|VARIDBlueprintFunctionLibrary|EndRendering))))

(event Input|KeyboardEvents|1
  (params (Key :type Key%20Structure :default "None"))
  ;[1 1 1] VARID Keyboard Actions
  (:Pressed
    (Class|VARIDBlueprintFunctionLibrary|ToggleFX 1)))

(event Input|KeyboardEvents|2
  (params (Key :type Key%20Structure :default "None"))
  ;[1 1 1] VARID Keyboard Actions
  (:Pressed
    (Class|VARIDBlueprintFunctionLibrary|ToggleFX 2)))

(event Input|KeyboardEvents|3
  (params (Key :type Key%20Structure :default "None"))
  ;[1 1 1] VARID Keyboard Actions
  (:Pressed
    (Class|VARIDBlueprintFunctionLibrary|ToggleFX 3)))

(event Input|KeyboardEvents|4
  (params (Key :type Key%20Structure :default "None"))
  ;[1 1 1] VARID Keyboard Actions
  (:Pressed
    (Class|VARIDBlueprintFunctionLibrary|ToggleFX 4)))

(event Input|KeyboardEvents|5
  (params (Key :type Key%20Structure :default "None"))
  ;[1 1 1] VARID Keyboard Actions
  (:Pressed
    (Class|VARIDBlueprintFunctionLibrary|ToggleFX 5)))

(event Input|KeyboardEvents|0
  (params (Key :type Key%20Structure :default "None"))
  ;[1 1 1] VARID Keyboard Actions
  (:Pressed
    (Class|VARIDBlueprintFunctionLibrary|ToggleFX)))

(event Input|KeyboardEvents|6
  (params (Key :type Key%20Structure :default "None"))
  ;[1 1 1] VARID Keyboard Actions
  (:Pressed
    (Class|VARIDBlueprintFunctionLibrary|ToggleFX 6)))

(event Input|KeyboardEvents|7
  (params (Key :type Key%20Structure :default "None"))
  ;[1 1 1] VARID Keyboard Actions
  (:Pressed
    (Class|VARIDBlueprintFunctionLibrary|ToggleFX 7)))

(event Input|KeyboardEvents|Period
  (params (Key :type Key%20Structure :default "None"))
  ;[1 1 1] VARID Keyboard Actions
  (:Pressed
    (Class|VARIDBlueprintFunctionLibrary|DisableAllFX)))

(event Input|KeyboardEvents|Comma
  (params (Key :type Key%20Structure :default "None"))
  ;[1 1 1] VARID Keyboard Actions
  (:Pressed
    (Class|VARIDBlueprintFunctionLibrary|EnableAllFX)))

(fn ConstructionScript)

(fn VARIDGetEyePositionsfromEyeTracker
  (bind _eye_tracking_sensitivity (Variables|Default|GetEye%20Tracking%20Sensitivity))
  (bind _outgazedata (Class|EyeTrackerFunctionLibrary|GetStereoGazeData))
  (return (Utilities|Struct|MakeVARIDEyeTracking (Math|Vector2D|MakeVector2D (* (.y (.lefteyedirection _outgazedata)) _eye_tracking_sensitivity) (* (* (.z (.lefteyedirection _outgazedata)) -1.0) _eye_tracking_sensitivity)) (Math|Vector2D|MakeVector2D (* (.y (.righteyedirection _outgazedata)) _eye_tracking_sensitivity) (* (* (.z (.righteyedirection _outgazedata)) -1.0) _eye_tracking_sensitivity)))))

(fn VARIDGetEyePositionsfromMouse
  (bind _returnvalue (Viewport|GetViewportSize))
  (bind _returnvalue_2 (Class|WidgetLayoutLibrary|GetViewportScale))
  (bind _returnvalue_3 (Class|WidgetLayoutLibrary|GetMousePositiononViewport))
  (return (Utilities|Struct|MakeVARIDEyeTracking (Math|Vector2D|MakeVector2D (- (Math|Float|NormalizetoRange (.x _returnvalue_3) 0.0 (/ (.x _returnvalue) _returnvalue_2)) 0.5) (- (Math|Float|NormalizetoRange (.y _returnvalue_3) 0.0 (/ (.y _returnvalue) _returnvalue_2)) 0.5)) (Math|Vector2D|MakeVector2D (- (Math|Float|NormalizetoRange (.x _returnvalue_3) 0.0 (/ (.x _returnvalue) _returnvalue_2)) 0.5) (- (Math|Float|NormalizetoRange (.y _returnvalue_3) 0.0 (/ (.y _returnvalue) _returnvalue_2)) 0.5)))))