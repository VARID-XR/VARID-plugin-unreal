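; BP_VARID_AR_Camera is an actor that starts a live video capture feed for the VARID AR camera view.
; On BeginPlay it opens the first enumerated capture device in a Media Player, selects the video track, applies a hardcoded format index and plays it.
; Steps are spaced by CameraDelay and gated on success, ending with the player's view target set to this actor.
; The C key reruns the sequence.
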(event EventBeginPlay
  (bind _outdevices (Class|MediaBlueprintFunctionLibrary|EnumerateVideoCaptureDevices -1))
  (Utilities|FlowControl|Delay (Variables|Default|GetCamera%20Delay))
  (bind _returnvalue (Class|MediaPlayer|OpenUrl (Variables|Default|GetMedia%20Player%20Ref) (.Url (Utilities|Struct|BreakMediaCaptureDevice (Utilities|Array|Get(acopy) _outdevices)))))
  (if _returnvalue
    (Utilities|FlowControl|Delay (Variables|Default|GetCamera%20Delay))
    (bind _returnvalue_2 (Class|MediaPlayer|SelectTrack (Variables|Default|GetMedia%20Player%20Ref) "Video"))
    (if _returnvalue_2
      (Utilities|FlowControl|Delay (Variables|Default|GetCamera%20Delay))
      (bind _returnvalue_3 (Class|MediaPlayer|SetTrackFormat (Variables|Default|GetMedia%20Player%20Ref) "Video" 0 323))
      (if _returnvalue_3
        (Utilities|FlowControl|Delay (Variables|Default|GetCamera%20Delay))
        (bind _returnvalue_4 (Media|MediaPlayer|Play (Variables|Default|GetMedia%20Player%20Ref) :!class /Script/MediaAssets.MediaPlayer))
        (if _returnvalue_4
          (Game|Player|SetViewTargetwithBlend (Game|GetPlayerController 0) self 0.0 "VTBlend_Linear" 0.0 false))))))

(event Input|KeyboardEvents|C
  (params (Key :type Key%20Structure :default "None"))
  (:Pressed
    (bind _outdevices (Class|MediaBlueprintFunctionLibrary|EnumerateVideoCaptureDevices -1))
    (Utilities|FlowControl|Delay (Variables|Default|GetCamera%20Delay))
    (bind _returnvalue (Class|MediaPlayer|OpenUrl (Variables|Default|GetMedia%20Player%20Ref) (.Url (Utilities|Struct|BreakMediaCaptureDevice (Utilities|Array|Get(acopy) _outdevices)))))
    (if _returnvalue
      (Utilities|FlowControl|Delay (Variables|Default|GetCamera%20Delay))
      (bind _returnvalue_2 (Class|MediaPlayer|SelectTrack (Variables|Default|GetMedia%20Player%20Ref) "Video"))
      (if _returnvalue_2
        (Utilities|FlowControl|Delay (Variables|Default|GetCamera%20Delay))
        (bind _returnvalue_3 (Class|MediaPlayer|SetTrackFormat (Variables|Default|GetMedia%20Player%20Ref) "Video" 0 323))
        (if _returnvalue_3
          (Utilities|FlowControl|Delay (Variables|Default|GetCamera%20Delay))
          (bind _returnvalue_4 (Media|MediaPlayer|Play (Variables|Default|GetMedia%20Player%20Ref) :!class /Script/MediaAssets.MediaPlayer))
          (if _returnvalue_4
            (Game|Player|SetViewTargetwithBlend (Game|GetPlayerController 0) self 0.0 "VTBlend_Linear" 0.0 false)))))))

(fn ConstructionScript)